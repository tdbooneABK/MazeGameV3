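; BP_Button is a pressure button for the maze game that reacts to overlaps on its CollisionSphere.
; On begin overlap it lights the ButtonBody material through a scalar parameter, sinks the body and calls OnButtonPress; end overlap reverses this and calls OnButtonRelease.
; An IsPressed flag blocks repeat triggers, but overlaps are not counted, so any actor leaving releases the button.
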(event `self.CollisionSphere.OnComponentBeginOverlap`
  (params (OverlappedComponent :type "PrimitiveComponent Object Reference") (OtherActor :type "Actor Object Reference") (OtherComp :type "PrimitiveComponent Object Reference") (OtherBodyIndex :type Integer) (bFromSweep :type Boolean) (SweepResult :type "HitResult Structure (by ref)"))
  (bind _buttonbody (`self.ButtonBody`))
  (if (not (`self.IsPressed`))
    (set `self.IsPressed` true)
    (`MeshComponent.SetScalarParameterValueOnMaterials` _buttonbody "ShouldLightUp" 1.0)
    (`SceneComponent.K2_SetWorldLocation` _buttonbody (- (`SceneComponent.K2_GetComponentLocation` _buttonbody) (0.0 0.0 10.0)) false false)
    (`self.OnButtonPress`)))

(event `self.CollisionSphere.OnComponentEndOverlap`
  (params (OverlappedComponent :type "PrimitiveComponent Object Reference") (OtherActor :type "Actor Object Reference") (OtherComp :type "PrimitiveComponent Object Reference") (OtherBodyIndex :type Integer))
  (bind _buttonbody (`self.ButtonBody`))
  (if (`self.IsPressed`)
    (set `self.IsPressed` false)
    (`MeshComponent.SetScalarParameterValueOnMaterials` _buttonbody "ShouldLightUp" 0.0)
    (`SceneComponent.K2_SetWorldLocation` _buttonbody (+ (`SceneComponent.K2_GetComponentLocation` _buttonbody) (0.0 0.0 10.0)) false false)
    (`self.OnButtonRelease`)))

(fn `UserConstructionScript`)